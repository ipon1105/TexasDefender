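; BP_InteractSeller is a seller actor that opens the in-game store when interacted with.
; Its BPIInteract event creates a Game_Store widget, adds it to the viewport and pauses the game.
; It contains no other active logic, as the BeginPlay, overlap and Tick events are disabled and the construction script only calls its parent.
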(event EventBeginPlay
  (|CallParentFunction) ; This node is disabled and will not be called.\nDrag off pins to build functionality.
)

(event Collision|EventActorBeginOverlap
  (params (OtherActor :type Actor%20Object%20Reference))
  (|CallParentFunction OtherActor) ; This node is disabled and will not be called.\nDrag off pins to build functionality.
)

(event EventTick
  (params (DeltaSeconds :type Float%20%28single-precision%29))
  (|CallParentFunction DeltaSeconds) ; This node is disabled and will not be called.\nDrag off pins to build functionality.
)

(event EventBPIInteract
  (bind _returnvalue (UserInterface|CreateWidget "/Game/UI/Game_Store.Game_Store_C"))
  (UserInterface|Viewport|AddtoViewport _returnvalue 0)
  (Game|SetGamePaused true))

(fn ConstructionScript
  (|CallParentFunction))